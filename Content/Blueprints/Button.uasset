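; Pressure button actor whose event graph is unfinished: Tick is empty and the press logic is disconnected.
; The construction script raises the mesh to ButtonOffset and sizes an arrow to match.
; The orphaned logic steps the mesh down or up within that offset, creating a DoorOpening sequence player on the down branch without playing it.
; The box overlap check meant to detect occupants is unused.
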(event `self.ReceiveTick`
  (params (DeltaSeconds :type "Float (single-precision)")))

(fn `UserConstructionScript`
  (bind _buttonoffset (`self.ButtonOffset`))
  (set `ArrowComponent.ArrowLength` _buttonoffset (`self.Arrow`))
  (`SceneComponent.K2_SetRelativeLocation` (`self.StaticMesh`) (`KismetMathLibrary.MakeVector` 0.0 0.0 _buttonoffset) false false))