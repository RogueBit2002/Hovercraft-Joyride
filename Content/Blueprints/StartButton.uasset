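; StartButton is a physical VR push button that plays the DoorOpening level sequence when fully pressed.
; Overlap by a VRPawn starts tracking its right motion controller, whichever component touched the button.
; Each tick projects controller travel onto the button's up vector, using the clamped absolute distance to depress it.
; At maximum travel it triggers the sequence, stops tracking and interpolates back to rest.
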(event `self.Button.OnComponentBeginOverlap`
  (params (OverlappedComponent :type "PrimitiveComponent Object Reference") (OtherActor :type "Actor Object Reference") (OtherComp :type "PrimitiveComponent Object Reference") (OtherBodyIndex :type Integer) (bFromSweep :type Boolean) (SweepResult :type "HitResult Structure (by ref)"))
  (bind _asvrpawn (cast `/Game/VRTemplate/Blueprints/VRPawn` OtherActor))
  (set `self.Tracking MC` (`/Game/VRTemplate/Blueprints/VRPawn.MotionControllerRight` _asvrpawn))
  (set `self.bIsTracking` true)
  (set `self.MC Initial Location` (`SceneComponent.K2_GetComponentLocation` (`self.Tracking MC`)))
  (set `self.Button Initial Location` (`SceneComponent.K2_GetComponentLocation` (`self.Button`))))

(event `self.ReceiveTick`
  (params (DeltaSeconds :type "Float (single-precision)"))
  (bind _button (`self.Button`))
  (bind _returnvalue (- (`self.Button Initial Location`) (* (`SceneComponent.GetUpVector` _button) (`self.Current Travel`))))
  (if (`self.bIsTracking`)
    (set `self.Current Travel` (`KismetMathLibrary.FClamp` (`KismetMathLibrary.Abs` (`KismetMathLibrary.VSize` (`KismetMathLibrary.ProjectVectorOnToVector` (- (`SceneComponent.K2_GetComponentLocation` (`self.Tracking MC`)) (`self.MC Initial Location`)) (`SceneComponent.GetUpVector` (`self.Button`))))) 0.0 (`self.Maximum Travel`)))
    (set `self.Button Current Location` _returnvalue)
    (`SceneComponent.K2_SetWorldLocation` _button _returnvalue false false)
    (if (>= (`self.Current Travel`) (`self.Maximum Travel`))
      (`self.Fully Pressed`)
      (`KismetSystemLibrary.PrintString` "Fully Pressed!"))
    (elif (`self.bIsReturning`)
      (bind _output_get (set `self.Button Current Location` (`KismetMathLibrary.VInterpTo` (`self.Button Current Location`) (`self.Button Initial Location`) (`GameplayStatics.GetWorldDeltaSeconds`) (`self.Button Return Speed`))))
      (`SceneComponent.K2_SetWorldLocation` (`self.Button`) _output_get false false)
      (if (`KismetMathLibrary.EqualExactly_VectorVector` (`self.Button Current Location`) (`self.Button Initial Location`))
        (set `self.bIsReturning` false)))))

(event `Fully Pressed`
  (bind _outactor (`LevelSequencePlayer.CreateLevelSequencePlayer` "/Game/DoorOpening.DoorOpening"))
  (`MovieSceneSequencePlayer.PlayTo` :`self` (`LevelSequenceActor.SequencePlayer` _outactor))
  (set `self.bIsTracking` false)
  (set `self.bIsReturning` true))

(fn `UserConstructionScript`)