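; Spline hover thruster that applies hover force to a receiver along a spline, holding it at a desired distance from surfaces.
; Each tick, evenly timed spline samples sphere-trace along the inverted up vector, splitting max force equally and keeping per-sample histories.
; The stabilizer term is zeroed on the first pass, before histories are valid.
; GetGrounding averages clamped normalized errors from those histories; a line-trace variant sits disconnected.
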(event `self.ReceiveBeginPlay`
  (set `self.Executed Once` false)
  (`parent.ReceiveBeginPlay`))

(event `self.ReceiveTick`
  (params (DeltaSeconds :type "Float (single-precision)"))
  (`self.Hover`)
  (`parent.ReceiveTick` DeltaSeconds))

(fn `Get Grounding`
  (returns (Grounding :type "Float (double-precision)"))
  (locals (Sum :type "Float (double-precision)") (Sum :type "Float (double-precision)"))
  (bind _histories (`self.Histories`))
  (set `local.Sum` 0.0)
  (for _array_element _histories
    (set `local.Sum` (+ (`KismetMathLibrary.FClamp` (+ (`.NormalizedError_7_7DCFFC5F4DB97B10416D289F8BC2795C` (break `/Game/Hover/Blueprints/HoverHistory` _array_element)) 1.0)) (`local.Sum`))))
  (return (/ (`local.Sum`) (`KismetMathLibrary.Conv_IntToDouble` (`KismetArrayLibrary.Array_Length` _histories)))))

(fn `Hover`
  (locals (`Current Index` :type Integer))
  (bind _samples (`self.Samples`))
  (bind _spline (`self.Spline`))
  (bind (_spring _stabilizer _compensator _maxcompensation) (break `/Game/Hover/Blueprints/HoverProperties` (`self.Properties`)))
  (bind _returnvalue (- _samples 1))
  (if (not (== (`self.Samples`) (`KismetArrayLibrary.Array_Length` (`self.Histories`))))
    (`KismetArrayLibrary.Array_Resize` (`self.Histories`) _samples))
  (for _index (range (+ _returnvalue 1))
    (bind _output_get (set `local.Current Index` _index))
    (bind _returnvalue_2 (/ (`KismetMathLibrary.Conv_IntToDouble` _output_get) (`KismetMathLibrary.Conv_IntToDouble` _returnvalue)))
    (bind _new_history (`/Game/Hover/Blueprints/HoverFunctionLibrary.Hover at Distance (SphereTrace)` (`self.Receiver`) (`SplineComponent.GetLocationAtTime` _spline _returnvalue_2 "World" false) (* (`SplineComponent.GetUpVectorAtTime` _spline _returnvalue_2 "World" false) -1.0) (`self.Desired Distance`) (make `/Game/Hover/Blueprints/HoverProperties` _spring (* _stabilizer (`KismetMathLibrary.Conv_BoolToDouble` (`self.Executed Once`))) _compensator _maxcompensation) (`|GetArrayItem` (`self.Histories`) (`local.Current Index`)) (/ (`self.Max Force`) (`KismetMathLibrary.Conv_IntToDouble` (`self.Samples`))) (`self.Radius`)))
    (`KismetArrayLibrary.Array_Set` (`self.Histories`) (`local.Current Index`) _new_history))
  (set `self.Executed Once` true))