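; Blueprint function library that hovers a component at a desired distance from surfaces using a PID controller.
; Line or sphere trace variants probe twice that distance on Visibility, converting hit time into normalized error.
; HoverInternal combines spring, clamped integral compensator and derivative stabilizer into a push-only force against the trace direction, applied at the origin.
; Callers carry state through the returned history; the sphere variant draws debug each call.
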(fn `Hover At Distance (LineTrace)`
  (params (Receiver :type "PrimitiveComponent Object Reference") (Origin :type "Vector Structure") (Direction :type "Vector Structure") (`Desired Distance` :type "Float (double-precision)") (Properties :type "/Game/Hover/Blueprints/HoverProperties Structure") (History :type "/Game/Hover/Blueprints/HoverHistory Structure") (`Max Force` :type "Float (double-precision)"))
  (returns (`New History` :type "/Game/Hover/Blueprints/HoverHistory Structure"))
  (bind _origin (`local.Origin`))
  ;[1 1 1] Cast
  (bind _outhit (`KismetSystemLibrary.LineTraceSingle` (`local.Receiver`) _origin (+ _origin (* (`local.Direction`) (* (`local.Desired Distance`) 2.0))) "TraceTypeQuery1"))
  (bind _new_history (`self.Hover Internal` (`local.Receiver`) (`local.Origin`) (`local.Direction`) (`local.Properties`) (`local.History`) (- (* (- 1.0 (`.Time` (`GameplayStatics.BreakHitResult` _outhit))) 2.0) 1.0) (`local.Max Force`)))
  (return _new_history))

(fn `Hover At Distance (SphereTrace)`
  (params (Receiver :type "PrimitiveComponent Object Reference") (Origin :type "Vector Structure") (Direction :type "Vector Structure") (`Desired Distance` :type "Float (double-precision)") (Properties :type "/Game/Hover/Blueprints/HoverProperties Structure") (History :type "/Game/Hover/Blueprints/HoverHistory Structure") (`Max Force` :type "Float (double-precision)") (Radius :type "Float (double-precision)"))
  (returns (`New History` :type "/Game/Hover/Blueprints/HoverHistory Structure"))
  (bind _origin (`local.Origin`))
  (bind _outhit (`KismetSystemLibrary.SphereTraceSingle` :`WorldContextObject` (`local.Receiver`) :`Start` _origin :`End` (+ _origin (* (`local.Direction`) (* (`local.Desired Distance`) 2.0))) :`Radius` (`local.Radius`) :`TraceChannel` "TraceTypeQuery1" :`DrawDebugType` "ForOneFrame"))
  (bind _new_history (`self.Hover Internal` (`local.Receiver`) (`local.Origin`) (`local.Direction`) (`local.Properties`) (`local.History`) (- (* (- 1.0 (`.Time` (`GameplayStatics.BreakHitResult` _outhit))) 2.0) 1.0) (`local.Max Force`)))
  (return _new_history))

(fn `Hover Internal`
  (params (Receiver :type "PrimitiveComponent Object Reference") (Origin :type "Vector Structure") (Direction :type "Vector Structure") (Properties :type "/Game/Hover/Blueprints/HoverProperties Structure") (History :type "/Game/Hover/Blueprints/HoverHistory Structure") (Error :type "Float (double-precision)") (`Max Force` :type "Float (double-precision)"))
  (returns (`New History` :type "/Game/Hover/Blueprints/HoverHistory Structure"))
  (locals (`New Integral` :type "Float (double-precision)"))
  (bind (_spring _stabilizer _compensator _maxcompensation) (break `/Game/Hover/Blueprints/HoverProperties` (`local.Properties`)))
  ;[1 1 1] Integral
  (bind _output_get (set `local.New Integral` (`KismetMathLibrary.FClamp` (+ (* (`local.Error`) (`GameplayStatics.GetWorldDeltaSeconds` null)) (`.Integral_6_F1BAB6264AF1FF77215DDDB037AFE902` (break `/Game/Hover/Blueprints/HoverHistory` (`local.History`)))) (* _maxcompensation 0.0) _maxcompensation)))
  ;[1 1 1] Apply Force
  (`PrimitiveComponent.AddForceAtLocation` (`local.Receiver`) (* (* (* (`KismetMathLibrary.Normal` (`local.Direction`)) -1.0) (`KismetMathLibrary.FMax` (+ (* (`KismetMathLibrary.FMax` (`local.Error`) -1.0) (`.Spring_2_AAB1E5D24176E9887900A5A165B5A202` (break `/Game/Hover/Blueprints/HoverProperties` (`local.Properties`)))) (* _output_get _compensator) (* (/ (- (`local.Error`) (`.NormalizedError_7_7DCFFC5F4DB97B10416D289F8BC2795C` (break `/Game/Hover/Blueprints/HoverHistory` (`local.History`)))) (`GameplayStatics.GetWorldDeltaSeconds` null)) (`.Stabilizer_12_0494E77648E609D901895C830727A131` (break `/Game/Hover/Blueprints/HoverProperties` (`local.Properties`))))))) (`local.Max Force`)) (`local.Origin`) "None")
  ;[1 1 1] Return
  (return (make `/Game/Hover/Blueprints/HoverHistory` (`local.Error`) (`local.New Integral`))))