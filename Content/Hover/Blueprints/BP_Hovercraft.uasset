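; Player-driven physics hovercraft, steered with W/A/D and braked with Space, with three spline thrusters wired to the root body and their splines at construction.
; Each tick, Drive applies forward thrust and horizontal friction, scaling thrust and braking by averaged, exponent-shaped HoverThruster grounding.
; Steer applies torque toward a target yaw rate, which also damps other rotation.
; Tick prints speed for debugging; Stabilize is never called.
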(event `self.ReceiveBeginPlay`)

(event `self.ReceiveTick`
  (params (DeltaSeconds :type "Float (single-precision)"))
  (bind _steering_input (`self.Steering Input`))
  (`self.Drive` (`self.Throttle Input`) (`self.Brake Input`) _steering_input)
  (`self.Steer` _steering_input)
  (bind _returnvalue (`PrimitiveComponent.GetPhysicsLinearVelocity` (`self.Root`) "None"))
  (`KismetSystemLibrary.PrintString` (`KismetStringLibrary.Conv_DoubleToString` (`KismetMathLibrary.VSize` _returnvalue))))

(event `Key|W`
  (params (Key :type "Key Structure"))
  (bind _throttle_input (`self.Throttle Input`))
  (:`Pressed`
    (`/Engine/EditorBlueprintResources/StandardMacros.IncrementFloat` _throttle_input))
  (:`Released`
    (`/Engine/EditorBlueprintResources/StandardMacros.DecrementFloat` _throttle_input)))

(event `Key|A`
  (params (Key :type "Key Structure"))
  (bind _steering_input (`self.Steering Input`))
  (:`Pressed`
    (`/Engine/EditorBlueprintResources/StandardMacros.DecrementFloat` _steering_input))
  (:`Released`
    (`/Engine/EditorBlueprintResources/StandardMacros.IncrementFloat` _steering_input)))

(event `Key|D`
  (params (Key :type "Key Structure"))
  (bind _steering_input (`self.Steering Input`))
  (:`Pressed`
    (`/Engine/EditorBlueprintResources/StandardMacros.IncrementFloat` _steering_input))
  (:`Released`
    (`/Engine/EditorBlueprintResources/StandardMacros.DecrementFloat` _steering_input)))

(event `Key|SpaceBar`
  (params (Key :type "Key Structure"))
  (bind _brake_input (`self.Brake Input`))
  (:`Pressed`
    (`/Engine/EditorBlueprintResources/StandardMacros.IncrementFloat` _brake_input))
  (:`Released`
    (`/Engine/EditorBlueprintResources/StandardMacros.DecrementFloat` _brake_input)))

(fn `Construct Spline Thruster`
  (params (Thruster :type "/Game/Hover/Blueprints/SplineHoverThruster Object Reference") (Receiver :type "PrimitiveComponent Object Reference") (Spline :type "SplineComponent Object Reference"))
  (`self.Construct Thruster` Thruster Receiver)
  (set `/Game/Hover/Blueprints/SplineHoverThruster.Spline` Spline Thruster))

(fn `Construct Thruster`
  (params (Thruster :type "/Game/Hover/Blueprints/SplineHoverThruster Object Reference") (Receiver :type "PrimitiveComponent Object Reference"))
  (set `/Game/Hover/Blueprints/HoverThruster.Receiver` Receiver Thruster))

(fn `Drive`
  (params (Throttle :type "Float (double-precision)") (Brake :type "Float (double-precision)") (Steering :type "Float (double-precision)"))
  (bind _linear_friction (`self.Linear Friction`))
  ;[1 1 1] Throttle
  (bind _grounding (`self.Get Grounding`))
  (`PrimitiveComponent.AddForce` (`self.Root`) (* (`SceneComponent.GetForwardVector` (`self.Root`)) (* (`KismetMathLibrary.Lerp` 0.25 1.0 _grounding) (* (`self.Max Speed`) (`self.Linear Friction`) (`local.Throttle`)))) "None" false)
  ;[1 1 1] Friction
  (bind _grounding_2 (`self.Get Grounding`))
  (bind _returnvalue (`PrimitiveComponent.GetPhysicsLinearVelocity` (`self.Root`) "None"))
  (`PrimitiveComponent.AddForce` (`self.Root`) (* (`KismetMathLibrary.MakeVector` (.x _returnvalue) (.y _returnvalue)) (* (`KismetMathLibrary.Lerp` _linear_friction (* _linear_friction (`self.Brake Multiplier`)) (* _grounding_2 (`local.Brake`))) -1.0)) "None" false))

(fn `Get Grounding`
  (returns (Grounding :type "Float (double-precision)"))
  (locals (Sum :type "Float (double-precision)"))
  (bind _returnvalue (`self.K2_GetComponentsByClass` "/Game/Hover/Blueprints/HoverThruster.HoverThruster_C"))
  (set `local.Sum` 0.0)
  (for _array_element _returnvalue
    (bind _grounding (`/Game/Hover/Blueprints/HoverThruster.Get Grounding` _array_element))
    (set `local.Sum` (+ _grounding (`local.Sum`))))
  (return (`KismetMathLibrary.MultiplyMultiply_FloatFloat` (/ (`local.Sum`) (`KismetMathLibrary.Conv_IntToDouble` (`KismetArrayLibrary.Array_Length` _returnvalue))) (`self.Grounding Exponent`))))

(fn `Stabilize`
  (params (Brake :type "Float (double-precision)"))
  (bind (_returnvalue_x _returnvalue_y _returnvalue_z) (`KismetMathLibrary.BreakVector` (`PrimitiveComponent.GetPhysicsAngularVelocityInDegrees` (`self.Root`) "None")))
  ;[1 1 1] Angular
  (`PrimitiveComponent.AddTorqueInDegrees` (`self.Root`) (* (`KismetMathLibrary.MakeVector` _returnvalue_x _returnvalue_y _returnvalue_z) (* (`self.Angular Friction`) -1.0)) "None" false))

(fn `Steer`
  (params (Steering :type "Float (double-precision)"))
  (bind _root (`self.Root`))
  (`PrimitiveComponent.AddTorqueInDegrees` (`self.Root`) (* (- (`KismetMathLibrary.TransformDirection` (`SceneComponent.K2_GetComponentToWorld` _root) (`KismetMathLibrary.MakeVector` 0.0 0.0 (* Steering (`self.Steering Speed`)))) (`PrimitiveComponent.GetPhysicsAngularVelocityInDegrees` _root "None")) (`self.Angular Friction`)) "None" false))

(fn `UserConstructionScript`
  (bind _root (`self.Root`))
  (`self.Construct Spline Thruster` (`self.Spline Thruster - Left`) _root (`self.Spline - Left Wing`))
  (`self.Construct Spline Thruster` (`self.Spline Thruster - Right`) _root (`self.Spline - Right Wing`))
  (`self.Construct Spline Thruster` (`self.Spline Thruster - Front`) _root (`self.Spline - Front`)))